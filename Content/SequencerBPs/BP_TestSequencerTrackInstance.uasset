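; BP_TestSequencerTrackInstance is a custom Sequencer track instance that shows storyboard images in the viewport.
; On initialize or input added, it lazily creates a WBP_StoryboardImage widget, which it removes when destroyed.
; Each added BP_TestSequencerSection passes its texture and match-size setting to that widget.
; Update and input-removed events only print debug strings, so the image persists after its section's input is removed.
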(event `self.K2_OnInitialize`
  (`KismetSystemLibrary.PrintString` "Initializing")
  (`self.CheckCreateStoryboardWidget`))

(event `self.K2_OnDestroyed`
  (bind _storyboardwidget (`self.StoryboardWidget`))
  (`/Engine/EditorBlueprintResources/StandardMacros.IsValid` _storyboardwidget
    (:`Is Valid`
      (`Widget.RemoveFromParent` _storyboardwidget))))

(event `self.K2_OnEndUpdateInputs`
  (`KismetSystemLibrary.PrintString` "On End Update Inputs"))

(event `self.K2_OnInputAdded`
  (params (Input :type "SequencerTrackInstanceInput Structure"))
  (bind _asbp_test_sequencer_section (cast `/Game/SequencerBPs/BP_TestSequencerSection` Input_Section))
  (`self.CheckCreateStoryboardWidget`)
  (`/Game/Widgets/WBP_StoryboardImage.SetImage` (`self.StoryboardWidget`) (`/Game/SequencerBPs/BP_TestSequencerSection.Texture` _asbp_test_sequencer_section) (`/Game/SequencerBPs/BP_TestSequencerSection.MatchImageSize` _asbp_test_sequencer_section)))

(event `self.K2_OnInputRemoved`
  (params (Input :type "SequencerTrackInstanceInput Structure"))
  (`KismetSystemLibrary.PrintString` "On Input Removed"))

(event `self.K2_OnUpdate`
  (`KismetSystemLibrary.PrintString` "On Update"))

(fn `CheckCreateStoryboardWidget`
  (`/Engine/EditorBlueprintResources/StandardMacros.IsValid` (`self.StoryboardWidget`)
    (:`Is Not Valid`
      (bind _returnvalue (`|CreateWidget` "/Game/Widgets/WBP_StoryboardImage.WBP_StoryboardImage_C" (`GameplayStatics.GetPlayerControllerFromID` 0)))
      (bind _output_get (set `self.StoryboardWidget` _returnvalue))
      (`UserWidget.AddToViewport` _output_get 0))))